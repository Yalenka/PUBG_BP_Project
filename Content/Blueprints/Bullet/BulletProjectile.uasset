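; Bullet projectile Blueprint that simulates velocity falloff over flight distance and leaves a bullet hole on impact.
; On movement component activation it records the launch location and applies the initial velocity.
; Each tick it lowers max speed by piecewise linear interpolation between reference velocities at 100, 300 and 500 meters.
; On hit it spawns a bullet hole decal at the impact point, then destroys itself.
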(event OnComponentActivated(ProjectileMovement)
  (params (Component :type Actor%20Component%20Object%20Reference) (bReset :type Boolean))
  ;[1 1 1] Set Initial Bullet Speed When Actor Gets Created
  (Variables|Default|SetInitLocation (Transformation|GetActorLocation))
  (bind _asprojectile_movement_component (Utilities|Casting|CastToProjectileMovementComponent Component))
  (Variables|/Script/Engine.ProjectileMovementComponent|SetInitialSpeed _asprojectile_movement_component (Variables|Default|GetInitVelocity))
  (Variables|/Script/Engine.ProjectileMovementComponent|SetMaxSpeed _asprojectile_movement_component (Variables|Default|GetInitVelocity)))

(event EventTick
  (params (DeltaSeconds :type Float%20%28single-precision%29))
  (Utilities|FlowControl|Sequence
    (:then_0
      ;[1 1 1] Get The flight distance in real time
      (Variables|Default|SetCurrentDistance (Math|Vector|VectorLength (- (Transformation|GetActorLocation) (Variables|Default|GetInitLocation))))
      ;[1 1 1] Reduce The Speed Value According To The Distance
      (if (<= (Variables|Default|GetCurrentDistance) 1e+04)
        (Variables|/Script/Engine.ProjectileMovementComponent|SetMaxSpeed (Variables|Default|GetProjectileMovement) (Math|Float|Lerp (Variables|Default|GetInitVelocity) (Variables|Default|Get100MVelocity) (/ (Variables|Default|GetCurrentDistance) 1e+04)))
        (elif (<= (Variables|Default|GetCurrentDistance) 3e+04)
          (Variables|/Script/Engine.ProjectileMovementComponent|SetMaxSpeed (Variables|Default|GetProjectileMovement) (Math|Float|Lerp (Variables|Default|Get100MVelocity) (Variables|Default|Get300MVelocity) (/ (- (Variables|Default|GetCurrentDistance) 1e+04) 2e+04)))
          (elif (<= (Variables|Default|GetCurrentDistance) 5e+04)
            (Variables|/Script/Engine.ProjectileMovementComponent|SetMaxSpeed (Variables|Default|GetProjectileMovement) (Math|Float|Lerp (Variables|Default|Get300MVelocity) (Variables|Default|Get500MVelocity) (/ (- (Variables|Default|GetCurrentDistance) 3e+04) 2e+04)))))))))

(event Collision|EventHit
  (params (MyComp :type Primitive%20Component%20Object%20Reference) (Other :type Actor%20Object%20Reference) (OtherComp :type Primitive%20Component%20Object%20Reference) (bSelfMoved :type Boolean) (HitLocation :type Vector :default "0, 0, 0") (HitNormal :type Vector :default "0, 0, 0") (NormalImpulse :type Vector :default "0, 0, 0") (Hit :type Hit%20Result%20Structure%20%28by%20ref%29))
  ;[1 1 1] Creates Bullet Hole
  (Game|SpawnActorfromClass "/Game/Blueprints/Bullet/BulletHoleDecal.BulletHoleDecal_C" (Math|Transform|MakeTransform HitLocation (Math|Transform|InverseTransformRotation (Transformation|GetWorldTransform OtherComp) (Transformation|GetWorldRotation MyComp))) "Undefined" 0 0)
  ;[1 1 1] Destroy Bullet Upon Collision
  (Actor|DestroyActor self))

(fn ConstructionScript)