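; Player state holding the player's loadout: two weapon slots, held gun, two ammo counts, health, energy, equipment, fashion and backpack items.
; Setters and add/remove functions fire change events, and weapon accessory updates are routed to the gun in the chosen slot or in hand.
; Ammo counts are mirrored into spawned backpack item actors, health and boost pickups stack by ID, and capacity checks compare item weight against default plus equipment capacity.
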(event EventBeginPlay)

(event EventTick
  (params (DeltaSeconds :type Float%20%28single-precision%29)))

(fn ConstructionScript)

(fn GetWeapon1
  (return (Variables|Items|GetWeapon1)))

(fn GetWeapon2
  (return (Variables|Items|GetWeapon2)))

(fn GetHoldGun
  (return (Variables|Items|GetHoldGun)))

(fn GetAmmo556
  (return (Variables|Items|GetAmmo556)))

(fn GetAmmo762
  (return (Variables|Items|GetAmmo762)))

(fn GetHealthPoint
  (return (Variables|Character|GetHealthPoint)))

(fn GetEnergyPoint
  (return (Variables|Character|GetEnergyPoint)))

(fn GetEquipments
  (return (Variables|Items|GetEquipments)))

(fn GetFashions
  (return (Variables|Items|GetFashions)))

(fn GetItems
  (return (Variables|Items|GetItemsInBackpack)))

(fn SetWeapon1
  (params (Weapon :type Item%20Weapon%20Object%20Reference))
  (bind _output_get (Variables|Items|SetWeapon1 Weapon))
  (Default|CallEventWeaponChanged _output_get "NewEnumerator0" false))

(fn SetWeapon2
  (params (Weapon :type Item%20Weapon%20Object%20Reference))
  (bind _output_get (Variables|Items|SetWeapon2 Weapon))
  (Default|CallEventWeaponChanged _output_get "NewEnumerator1" false))

(fn SetHoldGun
  (params (Weapon :type Item%20Weapon%20Object%20Reference))
  (bind _output_get (Variables|Items|SetHoldGun Weapon))
  (Utilities|IsValid _output_get
    (:Is%20Valid
      (Default|CallEventWeaponChanged _output_get (Variables|/Game/Blueprints/Items/Equipments/ItemWeapon.ItemWeapon_C|GetPosition _output_get) true))
    (:Is%20Not%20Valid
      (Default|CallEventWeaponChanged _output_get "NewEnumerator0" true))))

(fn SetAmmo556
  (params (Value :type Integer))
  (Variables|Items|SetAmmo556 Value)
  (Ammo|UpdateAmmoObject)
  (Default|CallEventAmmoChanged))

(fn SetHealthPoint
  (params (Value :type Float%20%28single-precision%29))
  (bind _output_get (Variables|Character|SetHealthPoint Value))
  (Default|CallEventHealthPointChanged _output_get))

(fn SetEnergyPoint
  (params (Value :type Float%20%28single-precision%29))
  (bind _output_get (Variables|Character|SetEnergyPoint Value))
  (Default|CallEventEnergyPointChanged _output_get))

(fn AddEquipment
  (params (Equipment :type Item%20Base%20Object%20Reference))
  (Utilities|Array|Add (Variables|Items|GetEquipments) Equipment)
  (Default|CallEventEquipmentsChanged Equipment true))

(fn AddFashion
  (params (Fashion :type Item%20Base%20Object%20Reference))
  (Utilities|Array|Add (Variables|Items|GetFashions) Fashion)
  (Default|CallEventFashionChanged Fashion true))

(fn AddItem
  (params (ItemIn :type Item%20Base%20Object%20Reference))
  (bind _itemtype (Variables|/Game/Blueprints/Items/ItemBase.ItemBase_C|GetItemType ItemIn))
  ;[1 1 1] If the item type is health or boost, and if there already an item of that type, the amount is added directly
  (if (or (Utilities|Enum|Equal(Enum) _itemtype "NewEnumerator3") (Utilities|Enum|Equal(Enum) _itemtype "NewEnumerator4"))
    (bind _array_element (Utilities|Array|ForEachLoopwithBreak (Variables|Items|GetItemsInBackpack) :!label _label)
      (:LoopBody
        (if (and (== (Variables|/Game/Blueprints/Items/ItemBase.ItemBase_C|GetItemType _array_element) (Variables|/Game/Blueprints/Items/ItemBase.ItemBase_C|GetItemType ItemIn)) (Utilities|Name|Equal(Name) (Variables|/Game/Blueprints/Items/ItemBase.ItemBase_C|GetID ItemIn) (Variables|/Game/Blueprints/Items/ItemBase.ItemBase_C|GetID _array_element)))
          (Variables|/Game/Blueprints/Items/ItemBase.ItemBase_C|SetAmount _array_element (+ (Variables|/Game/Blueprints/Items/ItemBase.ItemBase_C|GetAmount _array_element) (Variables|/Game/Blueprints/Items/ItemBase.ItemBase_C|GetAmount ItemIn)))
          (LocalVariables|SetisFound true)
          (Default|CallEventItemsChanged _array_element true)
          (goto _label Break)))
      (:Completed
        ;[1 1 1] Not a health or boost item, or no identical item type found, add to the item object.
        (if (not (LocalVariables|GetisFound)) :!label _label_2
          (Utilities|Array|Add (Variables|Items|GetItemsInBackpack) ItemIn)
          (Default|CallEventItemsChanged ItemIn true))))
    (else
      (goto _label_2))))

(fn RemoveEquipment
  (params (Equipment :type Item%20Base%20Object%20Reference))
  (bind _returnvalue (Utilities|Array|RemoveItem (Variables|Items|GetEquipments) Equipment))
  (Default|CallEventEquipmentsChanged Equipment false)
  (return _returnvalue))

(fn SetAmmo762
  (params (Value :type Integer))
  (Variables|Items|SetAmmo762 Value)
  (Ammo|UpdateAmmoObject)
  (Default|CallEventAmmoChanged))

(fn RemoveFashion
  (params (Equipment :type Item%20Base%20Object%20Reference))
  (bind _returnvalue (Utilities|Array|RemoveItem (Variables|Items|GetFashions) Equipment))
  (Default|CallEventFashionChanged Equipment false)
  (return _returnvalue))

(fn RemoveItem
  (params (Item :type Item%20Base%20Object%20Reference))
  (bind _returnvalue (Utilities|Array|RemoveItem (Variables|Items|GetItemsInBackpack) Item))
  (Default|CallEventItemsChanged Item false)
  (return _returnvalue))

(fn CheckBackpackCapacity
  (params (AddWeight :type Integer))
  ;[1 1 1] Determine if the capacity is sufficient after adding weight
  (if (<= (+ AddWeight (Backpack|ItemsTotalWeight)) (Backpack|BackpackTotalCapacity))
    (return true)
    (else
      (return false))))

(fn UpdateAmmoObject
  (for _array_element (Variables|Items|GetItemsInBackpack)
    ;[1 1 1] Find the ammo object in the backpack
    (if (Utilities|Enum|Equal(Enum) (Variables|/Game/Blueprints/Items/ItemBase.ItemBase_C|GetItemType _array_element) "NewEnumerator2")
      (if (Utilities|Name|Equal(Name) (Variables|/Game/Blueprints/Items/ItemBase.ItemBase_C|GetID _array_element) "1")
        (LocalVariables|SetAmmo1 _array_element)
        (else
          (LocalVariables|SetAmmo2 _array_element)))))
  (Utilities|FlowControl|Sequence
    (:then_0
      ;[1 1 1] The Number Of Bullets is greater than 0. If object exists, then set the number of objects
      (if (> (Getter|GetAmmo556) 0)
        (Utilities|IsValid (LocalVariables|GetAmmo1)
          (:Is%20Valid
            (Variables|/Game/Blueprints/Items/ItemBase.ItemBase_C|SetAmount (LocalVariables|GetAmmo1) (Getter|GetAmmo556)))
          (:Is%20Not%20Valid
            (bind _returnvalue (Game|SpawnActorfromClass "/Game/Blueprints/Items/Equipments/ItemAmmo.ItemAmmo_C" (Math|Transform|MakeTransform "0, 0, 0") "Undefined" 0 "1" (Default|GenerateSN (.AsMy%20Game%20Instance (Utilities|Casting|CastToMyGameInstance (Game|GetGameInstance)))) (Getter|GetAmmo556) 0))
            (ArrayAdd|AddItem _returnvalue)))
        (else
          ;[1 1 1] If the number of bullets is 0, the object is deleted
          (Utilities|IsValid (LocalVariables|GetAmmo1)
            (:Is%20Valid
              (ArrayRemove|RemoveItem (LocalVariables|GetAmmo1))
              (Actor|DestroyActor (LocalVariables|GetAmmo1)))))))
    (:then_1
      (if (> (Getter|GetAmmo762) 0)
        (Utilities|IsValid (LocalVariables|GetAmmo2)
          (:Is%20Valid
            (Variables|/Game/Blueprints/Items/ItemBase.ItemBase_C|SetAmount (LocalVariables|GetAmmo2) (Getter|GetAmmo762)))
          (:Is%20Not%20Valid
            (bind _returnvalue_2 (Game|SpawnActorfromClass "/Game/Blueprints/Items/Equipments/ItemAmmo.ItemAmmo_C" (Math|Transform|MakeTransform "0, 0, 0") "Undefined" 0 "2" (Default|GenerateSN (.AsMy%20Game%20Instance (Utilities|Casting|CastToMyGameInstance (Game|GetGameInstance)))) (Getter|GetAmmo762) 0))
            (ArrayAdd|AddItem _returnvalue_2)))
        (else
          (Utilities|IsValid (LocalVariables|GetAmmo2)
            (:Is%20Valid
              (ArrayRemove|RemoveItem (LocalVariables|GetAmmo2))
              (Actor|DestroyActor (LocalVariables|GetAmmo2)))))))))

(fn UpdateAmmoAmount
  (params (ID :type Name) (Add? :type Boolean) (Amount :type Integer))
  (if (== Amount 0)
    ;[1 1 1] If number is 0, the number of bullets is directly cleared
    (if (Utilities|Name|Equal(Name) ID "1")
      (Setter|SetAmmo556)
      (else
        (Setter|SetAmmo762)))
    (elif Add?
      (if (Utilities|Name|Equal(Name) ID "1")
        (Setter|SetAmmo556 (+ (Getter|GetAmmo556) Amount))
        (else
          (Setter|SetAmmo762 (+ (Getter|GetAmmo762) Amount))))
      (elif (Utilities|Name|Equal(Name) ID "1")
        (Setter|SetAmmo556 (- (Getter|GetAmmo556) Amount))
        (else
          (Setter|SetAmmo762 (- (Getter|GetAmmo762) Amount)))))))

(fn CheckReplaceBackpack
  (params (Item :type Item%20Base%20Object%20Reference))
  ;[1 1 1] Calculate the Total Weight of all Items
  (for _array_element (Getter|GetItems)
    (LocalVariables|SetItemsWeight (+ (Default|GetWeight _array_element) (LocalVariables|GetItemsWeight))))
  ;[1 1 1] Calculate if the new Backpack Capacity Is Enough
  (Utilities|FlowControl|Sequence
    (:then_0
      (Utilities|IsValid Item
        (:Is%20Valid
          (bind _returnvalue (Utilities|GetDataTableRow "/Game/Blueprints/Datas/DataTable/Items/DT_Item_Equipment.DT_Item_Equipment" (Variables|/Game/Blueprints/Items/ItemBase.ItemBase_C|GetID Item))
            (:then
              (LocalVariables|SetPickupCapacity (Utilities|Struct|BreakST_Item_Equipment _returnvalue)))))
        (:Is%20Not%20Valid
          (LocalVariables|SetPickupCapacity 0))))
    (:then_1
      (return (>= (+ (LocalVariables|GetPickupCapacity) (Variables|/Game/Blueprints/Gameplay/MyGameInstance.MyGameInstance_C|GetDefaultCapacity (.AsMy%20Game%20Instance (Utilities|Casting|CastToMyGameInstance (Game|GetGameInstance))))) (LocalVariables|GetItemsWeight))))))

(fn UpdateWeaponAcc
  (params (Position :type E_WeaponPosition%20Enum :default "NewEnumerator0") (AccType :type E_WeaponAccType%20Enum :default "NewEnumerator0") (ItemWeaponAcc :type Item%20Weapon%20Acc%20Object%20Reference))
  (bind _weapon1 (Variables|Items|GetWeapon1))
  (bind _weapon2 (Variables|Items|GetWeapon2))
  (Utilities|FlowControl|Sequence
    (:then_0
      ;[1 1 1] Get A Weapon Object
      (switch Utilities|FlowControl|Switch|SwitchonE_WeaponPosition Position
        (:NewEnumerator0
          (Utilities|IsValid _weapon1
            (:Is%20Valid
              (LocalVariables|SetWeapon _weapon1))
            (:Is%20Not%20Valid
              (LocalVariables|SetWeapon (Variables|Items|GetHoldGun) :!label _label))))
        (:NewEnumerator1
          (Utilities|IsValid _weapon2
            (:Is%20Valid
              (LocalVariables|SetWeapon _weapon2))
            (:Is%20Not%20Valid
              (goto _label))))))
    (:then_1
      ;[1 1 1] Save The Weapon Accessories And Update The Display
      (switch Utilities|FlowControl|Switch|SwitchonE_WeaponAccType AccType
        (:NewEnumerator0
          (Default|UpdateSight (LocalVariables|GetWeapon) ItemWeaponAcc))
        (:NewEnumerator1
          (Default|UpdateMuzzle (LocalVariables|GetWeapon) ItemWeaponAcc))
        (:NewEnumerator2
          (Default|UpdateForegrip (LocalVariables|GetWeapon) ItemWeaponAcc))
        (:NewEnumerator3
          (Default|UpdateMag (LocalVariables|GetWeapon) ItemWeaponAcc))
        (:NewEnumerator4
          (Default|UpdateButtstock (LocalVariables|GetWeapon) ItemWeaponAcc))))
    (:then_2
      ;[1 1 1] Call A Weapon Accessory Change Event
      (Default|CallEventWeaponAccChanged (not (Utilities|IsValid ItemWeaponAcc)) (LocalVariables|GetWeapon) ItemWeaponAcc AccType))))

(fn GetAmmoAmount
  (params (ID :type Name))
  (if (Utilities|Name|Equal(Name) ID "1")
    (return (Getter|GetAmmo556))
    (else
      (return (Getter|GetAmmo762)))))

(fn BackpackTotalCapacity
  (Utilities|FlowControl|Sequence
    (:then_0
      ;[1 1 1] Calculate Total Capacity
      (LocalVariables|SetTotalCapacity (Variables|/Game/Blueprints/Gameplay/MyGameInstance.MyGameInstance_C|GetDefaultCapacity (.AsMy%20Game%20Instance (Utilities|Casting|CastToMyGameInstance (Game|GetGameInstance)))))
      (for _array_element (Variables|Items|GetEquipments)
        (if (Utilities|Enum|Equal(Enum) (Variables|/Game/Blueprints/Items/ItemBase.ItemBase_C|GetItemType _array_element) "NewEnumerator7")
          (bind _returnvalue (Utilities|GetDataTableRow "/Game/Blueprints/Datas/DataTable/Items/DT_Item_Equipment.DT_Item_Equipment" (Variables|/Game/Blueprints/Items/ItemBase.ItemBase_C|GetID _array_element))
            (:then
              (LocalVariables|SetTotalCapacity (+ (LocalVariables|GetTotalCapacity) (Utilities|Struct|BreakST_Item_Equipment _returnvalue))))))))
    (:then_1
      (return (LocalVariables|GetTotalCapacity)))))

(fn ItemsTotalWeight
  (Utilities|FlowControl|Sequence
    (:then_0
      (for _array_element (Variables|Items|GetItemsInBackpack)
        (LocalVariables|SetItemsWeight (+ (Default|GetWeight _array_element) (LocalVariables|GetItemsWeight)))))
    (:then_1
      (return (LocalVariables|GetItemsWeight)))))