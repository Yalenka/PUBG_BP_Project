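; HUD Blueprint that creates the player's on-screen widgets at BeginPlay and exposes functions to control some of them.
; Crosshairs, user info, countdown and direction widgets stay visible, while action tips, message tips, item-use and parachute widgets start hidden.
; Show functions pass text or a time to their widget before revealing it; message and item-use widgets sit at a higher Z-order.
; Message tips has no hide function here.
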(event EventBeginPlay
  (Utilities|FlowControl|Sequence
    (:then_0
      (bind _returnvalue (UserInterface|CreateWidget "/Game/Blueprints/UI/MainUI/CrosshairsUI.CrosshairsUI_C"))
      (UserInterface|Viewport|AddtoViewport _returnvalue 0))
    (:then_1
      (bind _returnvalue_2 (UserInterface|CreateWidget "/Game/Blueprints/UI/MainUI/ActionTipsUI.ActionTipsUI_C"))
      (bind _output_get (Variables|Default|SetActionTipsUI _returnvalue_2))
      (Widget|SetVisibility _output_get "Hidden")
      (UserInterface|Viewport|AddtoViewport _output_get 0))
    (:then_2
      (bind _returnvalue_3 (UserInterface|CreateWidget "/Game/Blueprints/UI/MainUI/MessageTipsUI.MessageTipsUI_C"))
      (bind _output_get_2 (Variables|Default|SetMessageTipsUI _returnvalue_3))
      (Widget|SetVisibility _output_get_2 "Hidden")
      (UserInterface|Viewport|AddtoViewport _output_get_2 1))
    (:then_3
      (bind _returnvalue_4 (UserInterface|CreateWidget "/Game/Blueprints/UI/MainUI/UserInfoUI.UserInfoUI_C"))
      (bind _output_get_3 (Variables|Default|SetUserInfoUI _returnvalue_4))
      (UserInterface|Viewport|AddtoViewport _output_get_3 0))
    (:then_4
      (bind _returnvalue_5 (UserInterface|CreateWidget "/Game/Blueprints/UI/MainUI/CountDownUI.CountDownUI_C"))
      (UserInterface|Viewport|AddtoViewport _returnvalue_5 0))
    (:then_5
      (bind _returnvalue_6 (UserInterface|CreateWidget "/Game/Blueprints/UI/MainUI/DirectionUI.DirectionUI_C"))
      (UserInterface|Viewport|AddtoViewport _returnvalue_6 0))
    (:then_6
      (bind _returnvalue_7 (UserInterface|CreateWidget "/Game/Blueprints/UI/MainUI/UseItemUI.UseItemUI_C"))
      (bind _output_get_4 (Variables|Default|SetUseItemUI _returnvalue_7))
      (Widget|SetVisibility _output_get_4 "Hidden")
      (UserInterface|Viewport|AddtoViewport _output_get_4 1))
    (:then_7
      (bind _returnvalue_8 (UserInterface|CreateWidget "/Game/Blueprints/UI/Particles/ParticlesUI.ParticlesUI_C"))
      (bind _output_get_5 (Variables|Default|SetParachuteUI _returnvalue_8))
      (Widget|SetVisibility _output_get_5 "Hidden")
      (UserInterface|Viewport|AddtoViewport _output_get_5 0))))

(fn ConstructionScript)

(fn ShowActionTipsUI
  (params (Info :type Text))
  (Default|SetInfo (Variables|Default|GetActionTipsUI) Info)
  (Widget|SetVisibility (Variables|Default|GetActionTipsUI) "Visible"))

(fn HideActionTipsUI
  (Widget|SetVisibility (Variables|Default|GetActionTipsUI) "Hidden"))

(fn ShowMessageTipsUI
  (params (Info :type Text))
  (Default|SetInfo (Variables|Default|GetMessageTipsUI) Info)
  (Widget|SetVisibility (Variables|Default|GetMessageTipsUI) "Visible"))

(fn ShowUseItemUI
  (params (Time :type Float%20%28single-precision%29))
  (Default|Start (Variables|Default|GetUseItemUI) Time)
  (Widget|SetVisibility (Variables|Default|GetUseItemUI) "Visible"))

(fn HideUseItemUI
  (Widget|SetVisibility (Variables|Default|GetUseItemUI) "Hidden"))

(fn ShowParachuteUI
  (Widget|SetVisibility (Variables|Default|GetParachuteUI) "Visible"))

(fn HideParachuteUI
  (Widget|SetVisibility (Variables|Default|GetParachuteUI) "Hidden"))