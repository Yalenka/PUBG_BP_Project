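; Player character for a shooter, handling modular clothing, visible gear, stance-based montages and aiming cameras.
; Data table fashion rows swap master-posed body meshes and set skin material masks that fit the clothing.
; Weapons and equipment from MyPlayerState attach to mesh sockets.
; Aiming eases the camera along a timeline, then can switch to first-person arms positioned per weapon and sight; debug keys spawn attachments and an airplane.
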(event Custom|HoldAiming
  (params (Forward :type Boolean))
  ;[1 1 1] Aiming
  (Components|Timeline|SetPlayRate (Variables|Default|GetTL_HoldAiming) 1.0)
  (if Forward
    (bind _percent (Timeline|TL_HoldAiming Play)
      (:Update
        (Transformation|SetRelativeLocation (Variables|Default|GetCamera) (Math|Vector|Lerp(Vector) "0, 0, 0" "100.000000,5.000000,-30.000000" _percent) false false))
      (:Finished
        (Utilities|FlowControl|Sequence
          (:then_0
            (if (Variables|CharacterState|GetisSightAiming)
              (Aiming|SwitchCamera true)))
          (:then_1
            (if (not Forward)
              (Variables|CharacterState|SetisAiming false))))))
    (else
      (Timeline|TL_HoldAiming Reverse))))

(event EventBeginPlay
  ;[1 1 1] Create Object References
  (bind _asmy_player_state (Utilities|Casting|CastToMyPlayerState (Variables|GetPlayerState)))
  (Variables|Default|SetMyPlayerStateRef _asmy_player_state)
  (bind _asmy_game_instance (Utilities|Casting|CastToMyGameInstance (Game|GetGameInstance)))
  (Variables|Default|SetMyGameInstanceRef _asmy_game_instance))

(event Input|KeyboardEvents|3
  (params (Key :type Key%20Structure :default "None"))
  (:Pressed
    (bind (_startingpoint _endpoint) (Default|RandomRoute (.AsMy%20Game%20Mode (Utilities|Casting|CastToMyGameMode (Game|GetGameMode)))))
    (bind _returnvalue (Game|SpawnActorfromClass "/Game/Blueprints/AirNav/Airplane.Airplane_C" (Math|Transform|MakeTransform "0, 0, 0") "Undefined" 0 _startingpoint _endpoint 0))
    (Default|StartFlying (.AsMy%20Player%20Controller (Utilities|Casting|CastToMyPlayerController (Game|GetPlayerController 0))) _returnvalue)))

(event Input|KeyboardEvents|L
  (params (Key :type Key%20Structure :default "None"))
  ;[1 1 1] Scope testing
  (:Pressed
    (bind _returnvalue (Game|SpawnActorfromClass "/Game/Blueprints/Items/Equipments/ItemWeaponAcc.ItemWeaponAcc_C" (Math|Transform|MakeTransform "0, 0, 0") "Undefined" 0 "1" "111" 1 0))
    (Default|EquipAccessories (.AsMy%20Player%20Controller (Utilities|Casting|CastToMyPlayerController (Pawn|GetController))) _returnvalue false (Default|GetHoldGun (Variables|Default|GetMyPlayerStateRef)))))

(event Input|KeyboardEvents|K
  (params (Key :type Key%20Structure :default "None"))
  ;[1 1 1] Scope testing
  (:Pressed
    (bind _returnvalue (Game|SpawnActorfromClass "/Game/Blueprints/Items/Equipments/ItemWeaponAcc.ItemWeaponAcc_C" (Math|Transform|MakeTransform "0, 0, 0") "Undefined" 0 "18" "111" 1 0))
    (Default|EquipAccessories (.AsMy%20Player%20Controller (Utilities|Casting|CastToMyPlayerController (Pawn|GetController))) _returnvalue false (Default|GetHoldGun (Variables|Default|GetMyPlayerStateRef)))))

(fn ConstructionScript
  (SkeletalMesh|InitSkeletalMesh))

(fn MouseTurn
  (params (AxisValue :type Float%20%28single-precision%29))
  (Pawn|Input|AddControllerYawInput AxisValue))

(fn MouseLookUp
  (params (AxisValue :type Float%20%28single-precision%29))
  (Pawn|Input|AddControllerPitchInput AxisValue))

(fn InitSkeletalMesh
  (Utilities|FlowControl|Sequence
    (:then_0
      ;[1 1 1] Create Skin Material
      (bind _returnvalue (Rendering|Material|CreateDynamicMaterialInstance "/Game/Assets/Humans/Female/Materials/Skin/M_MT_Skin.M_MT_Skin" "None" "None" :!class /Script/Engine.KismetMaterialLibrary))
      (bind _output_get (Variables|SkeletalMesh|SetSkin%20Mat%20Ref _returnvalue))
      (Rendering|Material|SetMaterialbyName (Variables|Character|GetMesh) "skin" _output_get))
    (:then_1
      ;[1 1 1] Set Master Pose.
      (Class|SkinnedMeshComponent|SetMasterPoseComponent (Variables|Default|GetSKM_UnderwearTop) (Variables|Character|GetMesh) false))
    (:then_2
      ;[1 1 1] Attach Hair
      (Transformation|AttachComponentToComponent (Variables|Default|GetSKM_Hair) (Variables|Character|GetMesh) "Head" "KeepWorld" "KeepWorld" "KeepWorld" true))
    (:then_3
      ;[1 1 1] initial Skeletal mesh
      (SkeletalMesh|ReplaceSkeletalMesh "NewEnumerator0" "0"))))

(fn ReplaceSkeletalMesh
  (params (FashionType :type E_FashionType%20Enum :default "NewEnumerator0") (Name :type Name))
  (bind _mesh (Variables|Character|GetMesh))
  (Utilities|FlowControl|Sequence
    (:then_0
      (bind (_skeletalmesh _masktexture) (SkeletalMesh|GetFashionDatas Name))
      (LocalVariables|SetSKM _skeletalmesh)
      (LocalVariables|SetMask _masktexture)
      ;[1 1 1] Replace SkeletalMesh
      (switch Utilities|FlowControl|Switch|SwitchonE_FashionType FashionType
        (:NewEnumerator0
          (Class|SkinnedMeshComponent|SetSkeletalMesh (Variables|Default|GetSKM_ClothTop) (LocalVariables|GetSKM) true)
          ;[1 1 1] Set Mask
          (Rendering|Material|SetTextureParameterValue (Variables|SkeletalMesh|GetSkin%20Mat%20Ref) "Mask Top" (LocalVariables|GetMask))
          ;[1 1 1] Whole Special Modify
          (if (!= (LocalVariables|GetSKM) 0)
            (Class|SkinnedMeshComponent|SetSkeletalMesh (Variables|Default|GetSKM_Whole) 0 true)))
        (:NewEnumerator1
          (Class|SkinnedMeshComponent|SetSkeletalMesh (Variables|Default|GetSKM_ClothBottom) (LocalVariables|GetSKM) true)
          (Rendering|Material|SetTextureParameterValue (Variables|SkeletalMesh|GetSkin%20Mat%20Ref) "Mask Bottom" (LocalVariables|GetMask))
          (if (!= (LocalVariables|GetSKM) 0)
            (Class|SkinnedMeshComponent|SetSkeletalMesh (Variables|Default|GetSKM_Whole) 0 true)))
        (:NewEnumerator2
          (Class|SkinnedMeshComponent|SetSkeletalMesh (Variables|Default|GetSKM_Whole) (LocalVariables|GetSKM) true)
          (Rendering|Material|SetTextureParameterValue (Variables|SkeletalMesh|GetSkin%20Mat%20Ref) "Mask Top" (LocalVariables|GetMask))
          (if (!= (LocalVariables|GetSKM) 0)
            (Class|SkinnedMeshComponent|SetSkeletalMesh (Variables|Default|GetSKM_ClothTop) 0 true)
            (Class|SkinnedMeshComponent|SetSkeletalMesh (Variables|Default|GetSKM_ClothBottom) 0 true)))
        (:NewEnumerator3
          (Class|SkinnedMeshComponent|SetSkeletalMesh (Variables|Default|GetSKM_Shoes) (LocalVariables|GetSKM) true)
          (Utilities|IsValid (LocalVariables|GetSKM)
            (:Is%20Valid
              (Rendering|Material|SetTextureParameterValue (Variables|SkeletalMesh|GetSkin%20Mat%20Ref) "Mask Foot" (LocalVariables|GetMask))
              ;[1 1 1] Fix Character Height when wearing shoes
              (Transformation|SetRelativeLocation _mesh (Math|Vector|MakeVector 0.0 0.0 -96.900002) false false))
            (:Is%20Not%20Valid
              (Rendering|Material|SetTextureParameterValue (Variables|SkeletalMesh|GetSkin%20Mat%20Ref) "Mask Foot" "/Game/Assets/Humans/Female/Textures/System/TX_Empty_white.TX_Empty_white")
              (Transformation|SetRelativeLocation _mesh (Math|Vector|MakeVector 0.0 0.0 -97.599998) false false))))))
    (:then_1
      ;[1 1 1] Set the default SkeletalMesh and Mask
      (Utilities|IsValid (Variables|/Script/Engine.SkinnedMeshComponent|GetSkeletalMesh (Variables|Default|GetSKM_Whole))
        (:Is%20Valid
          (Rendering|Material|SetTextureParameterValue (Variables|SkeletalMesh|GetSkin%20Mat%20Ref) "Mask Bottom" "/Game/Assets/Humans/Female/Textures/System/TX_Empty_white.TX_Empty_white"))
        (:Is%20Not%20Valid
          (Utilities|FlowControl|Sequence
            (:then_0
              (Utilities|IsValid (Variables|/Script/Engine.SkinnedMeshComponent|GetSkeletalMesh (Variables|Default|GetSKM_ClothTop))
                (:Is%20Not%20Valid
                  (bind (_skeletalmesh_2 _masktexture_2) (SkeletalMesh|GetFashionDatas "1"))
                  (Class|SkinnedMeshComponent|SetSkeletalMesh (Variables|Default|GetSKM_ClothTop) _skeletalmesh_2 true)
                  (Rendering|Material|SetTextureParameterValue (Variables|SkeletalMesh|GetSkin%20Mat%20Ref) "Mask Top" _masktexture_2))))
            (:then_1
              (Utilities|IsValid (Variables|/Script/Engine.SkinnedMeshComponent|GetSkeletalMesh (Variables|Default|GetSKM_ClothBottom))
                (:Is%20Not%20Valid
                  (bind (_skeletalmesh_3 _masktexture_3) (SkeletalMesh|GetFashionDatas "4"))
                  (Class|SkinnedMeshComponent|SetSkeletalMesh (Variables|Default|GetSKM_ClothBottom) _skeletalmesh_3 true)
                  (Rendering|Material|SetTextureParameterValue (Variables|SkeletalMesh|GetSkin%20Mat%20Ref) "Mask Bottom" _masktexture_3))))))))))

(fn GetFashionDatas
  (params (ID :type Name))
  (bind _returnvalue (Utilities|GetDataTableRow "/Game/Blueprints/Datas/DataTable/Items/DT_Item_Fashion.DT_Item_Fashion" ID)
    (:then
      (return (.SkeletalMesh (Utilities|Struct|BreakST_Item_Fashion _returnvalue)) (.MaskTexture (Utilities|Struct|BreakST_Item_Fashion _returnvalue))))
    (:RowNotFound
      (return 0 0))))

(fn UpdateWeaponDisplay
  (params (HoldSocket :type Name))
  (bind _myplayerstateref (Variables|Default|GetMyPlayerStateRef))
  (bind _myplayerstateref_2 (Variables|Default|GetMyPlayerStateRef))
  (bind _myplayerstateref_3 (Variables|Default|GetMyPlayerStateRef))
  (bind _weapon (Default|GetWeapon1 _myplayerstateref))
  (bind _weapon_2 (Default|GetWeapon2 _myplayerstateref_3))
  (bind _weapon_3 (Default|GetHoldGun _myplayerstateref_2))
  (Utilities|FlowControl|Sequence
    (:then_0
      (if (not (Variables|CharacterState|GetisSightAiming))
        ;[1 1 1] Update The Handheld Weapon Display
        (if (Utilities|Name|NotEqual(Name) HoldSocket "None")
          (Utilities|IsValid _weapon_3
            (:Is%20Valid
              (ChangingItems|Attach _weapon_3 HoldSocket))))))
    (:then_1
      ;[1 1 1] Update Weapon Display
      (Utilities|FlowControl|Sequence
        (:then_0
          (for _array_element (Default|GetEquipments (Variables|Default|GetMyPlayerStateRef))
            (if (Utilities|Enum|Equal(Enum) (Variables|/Game/Blueprints/Items/ItemBase.ItemBase_C|GetItemType _array_element) "NewEnumerator7")
              (LocalVariables|SetisEquipBackpack true))))
        (:then_1
          (Utilities|IsValid (Default|GetWeapon1 (Variables|Default|GetMyPlayerStateRef))
            (:Is%20Valid
              (if (LocalVariables|GetisEquipBackpack)
                (ChangingItems|Attach _weapon (Variables|/Game/Blueprints/Gameplay/MyGameInstance.MyGameInstance_C|GetBackLeftBName (Variables|Default|GetMyGameInstanceRef)))
                (else
                  (ChangingItems|Attach _weapon (Variables|/Game/Blueprints/Gameplay/MyGameInstance.MyGameInstance_C|GetBackLeftNName (Variables|Default|GetMyGameInstanceRef))))))))
        (:then_2
          (Utilities|IsValid (Default|GetWeapon2 (Variables|Default|GetMyPlayerStateRef))
            (:Is%20Valid
              (if (LocalVariables|GetisEquipBackpack)
                (ChangingItems|Attach _weapon_2 (Variables|/Game/Blueprints/Gameplay/MyGameInstance.MyGameInstance_C|GetBackRightBName (Variables|Default|GetMyGameInstanceRef)))
                (else
                  (ChangingItems|Attach _weapon_2 (Variables|/Game/Blueprints/Gameplay/MyGameInstance.MyGameInstance_C|GetBackRightNName (Variables|Default|GetMyGameInstanceRef))))))))))))

(fn Attach
  (params (Item :type Item%20Base%20Object%20Reference) (SocketName :type Name))
  (Transformation|SetActorTransform Item (Transformation|GetSocketTransform (Variables|Character|GetMesh) SocketName "RTS_World"))
  (Transformation|AttachComponentToComponent Item (Variables|Character|GetMesh) SocketName "SnapToTarget" "KeepWorld" "KeepRelative" true))

(fn UpdateEquipmentDisplay
  (bind _skm_hair (Variables|Default|GetSKM_Hair))
  (Utilities|FlowControl|Sequence
    (:then_0
      (for _array_element (Default|GetEquipments (Variables|Default|GetMyPlayerStateRef))
        (bind _output_get (LocalVariables|SetItem _array_element))
        (switch Utilities|FlowControl|Switch|SwitchonE_ItemType (Variables|/Game/Blueprints/Items/ItemBase.ItemBase_C|GetItemType _output_get)
          (:NewEnumerator5
            (ChangingItems|Attach (LocalVariables|GetItem) (Variables|/Game/Blueprints/Gameplay/MyGameInstance.MyGameInstance_C|GetHelmetName (Variables|Default|GetMyGameInstanceRef)))
            (LocalVariables|SetHasHelmet true))
          (:NewEnumerator6
            (ChangingItems|Attach (LocalVariables|GetItem) (Variables|/Game/Blueprints/Gameplay/MyGameInstance.MyGameInstance_C|GetVestName (Variables|Default|GetMyGameInstanceRef))))
          (:NewEnumerator7
            (ChangingItems|Attach (LocalVariables|GetItem) (Variables|/Game/Blueprints/Gameplay/MyGameInstance.MyGameInstance_C|GetBackpackName (Variables|Default|GetMyGameInstanceRef)))))))
    (:then_1
      (if (LocalVariables|GetHasHelmet)
        (Rendering|SetVisibility _skm_hair false false)
        (else
          (Rendering|SetVisibility _skm_hair true false))))))

(fn ClearFashion
  (SkeletalMesh|ReplaceSkeletalMesh "NewEnumerator0" "0")
  (SkeletalMesh|ReplaceSkeletalMesh "NewEnumerator1" "0")
  (SkeletalMesh|ReplaceSkeletalMesh "NewEnumerator2" "0")
  (SkeletalMesh|ReplaceSkeletalMesh "NewEnumerator3" "0"))

(fn UpdateFashionDisplay
  (SkeletalMesh|ClearFashion)
  (for _array_element (Default|GetFashions (Variables|Default|GetMyPlayerStateRef))
    (bind _asitem_fashion (Utilities|Casting|CastToItemFashion _array_element))
    (SkeletalMesh|ReplaceSkeletalMesh (Variables|/Game/Blueprints/Items/Equipments/ItemFashion.ItemFashion_C|GetFashionType _asitem_fashion) (Variables|/Game/Blueprints/Items/ItemBase.ItemBase_C|GetID _asitem_fashion))))

(fn PlayMontage
  (params (MontageType :type E_MontageType%20Enum :default "NewEnumerator0") (PlayRate :type Float%20%28single-precision%29))
  (Variables|Animation|SetPlayingMontageType MontageType)
  (Variables|Animation|SetisPlayingMontage true)
  (if (Variables|CharacterPose|GetisProne)
    ;[1 1 1] Prone Montage Animation
    (switch Utilities|FlowControl|Switch|SwitchonE_MontageType MontageType
      (:NewEnumerator0
        (Animation|PlayAnimMontage "/Game/Blueprints/Character/Montage/AS_Prone_Equip_Montage.AS_Prone_Equip_Montage" 1.0 "None"))
      (:NewEnumerator1
        (Animation|PlayAnimMontage "/Game/Blueprints/Character/Montage/AS_Prone_UnEquip_Montage.AS_Prone_UnEquip_Montage" 1.0 "None"))
      (:NewEnumerator2
        (Animation|PlayAnimMontage "/Game/Blueprints/Character/Montage/AS_Prone_Reload_Montage.AS_Prone_Reload_Montage" PlayRate "None"))
      (:NewEnumerator3
        (Animation|PlayAnimMontage "/Game/Blueprints/Character/Montage/AS_Prone_Reload_Montage.AS_Prone_Reload_Montage" 1.0 "ReloadBullet"))
      (:NewEnumerator4
        (Animation|PlayAnimMontage "/Game/Blueprints/Character/Montage/AS_Rifle_Prone_Fire_Montage.AS_Rifle_Prone_Fire_Montage" 0.466 "None"))
      (:NewEnumerator5
        (Animation|PlayAnimMontage "/Game/Blueprints/Character/Montage/AS_Prone_Use_Object_Montage.AS_Prone_Use_Object_Montage" 1.0 "None")))
    (elif (Variables|CharacterPose|GetisCrouching)
      ;[1 1 1] Crouch Montage Animation
      (switch Utilities|FlowControl|Switch|SwitchonE_MontageType MontageType
        (:NewEnumerator0
          (Animation|PlayAnimMontage "/Game/Blueprints/Character/Montage/AS_Crouch_Equip_Montage.AS_Crouch_Equip_Montage" 1.0 "None"))
        (:NewEnumerator1
          (Animation|PlayAnimMontage "/Game/Blueprints/Character/Montage/AS_Crouch_UnEquip_Montage.AS_Crouch_UnEquip_Montage" 1.0 "None"))
        (:NewEnumerator2
          (Animation|PlayAnimMontage "/Game/Blueprints/Character/Montage/AS_Stand_Reload_Montage.AS_Stand_Reload_Montage" PlayRate "None"))
        (:NewEnumerator3
          (Animation|PlayAnimMontage "/Game/Blueprints/Character/Montage/AS_Stand_Reload_Montage.AS_Stand_Reload_Montage" 1.0 "ReloadBullet"))
        (:NewEnumerator4
          (Animation|PlayAnimMontage "/Game/Blueprints/Character/Montage/AS_Rifle_Crouch_Fire_Montage.AS_Rifle_Crouch_Fire_Montage" 2.0 "None"))
        (:NewEnumerator5
          (Animation|PlayAnimMontage "/Game/Blueprints/Character/Montage/AS_Crouch_Use_Object_Montage.AS_Crouch_Use_Object_Montage" 1.0 "None")))
      (else
        ;[1 1 1] Stand Montage Animation
        (switch Utilities|FlowControl|Switch|SwitchonE_MontageType MontageType
          (:NewEnumerator0
            (Animation|PlayAnimMontage "/Game/Blueprints/Character/Montage/AS_Stand_Equip_Montage.AS_Stand_Equip_Montage" 1.0 "None"))
          (:NewEnumerator1
            (Animation|PlayAnimMontage "/Game/Blueprints/Character/Montage/AS_Stand_UnEquip_Montage.AS_Stand_UnEquip_Montage" 1.0 "None"))
          (:NewEnumerator2
            (Animation|PlayAnimMontage "/Game/Blueprints/Character/Montage/AS_Stand_Reload_Montage.AS_Stand_Reload_Montage" PlayRate "None"))
          (:NewEnumerator3
            (Animation|PlayAnimMontage "/Game/Blueprints/Character/Montage/AS_Stand_Reload_Montage.AS_Stand_Reload_Montage" 1.0 "ReloadBullet"))
          (:NewEnumerator4
            (Animation|PlayAnimMontage "/Game/Blueprints/Character/Montage/AS_Rifle_Stand_Fire_Montage.AS_Rifle_Stand_Fire_Montage" 2.0 "None"))
          (:NewEnumerator5
            (Animation|PlayAnimMontage "/Game/Blueprints/Character/Montage/AS_Stand_Use_Object_Montage.AS_Stand_Use_Object_Montage" 1.0 "None")))))))

(fn SwitchCamera
  (params (IsFirst :type Boolean))
  (bind _myplayerstateref (Variables|Default|GetMyPlayerStateRef))
  (bind _myplayerstateref_2 (Variables|Default|GetMyPlayerStateRef))
  (bind _fpscamera (Variables|Default|GetFPSCamera))
  (bind _myplayerstateref_3 (Variables|Default|GetMyPlayerStateRef))
  (bind _weapon (Default|GetHoldGun _myplayerstateref))
  (bind _weapon_2 (Default|GetHoldGun _myplayerstateref_2))
  (bind _weapon_3 (Default|GetHoldGun _myplayerstateref_3))
  (bind _accsightobj (Variables|/Game/Blueprints/Items/Equipments/ItemWeapon.ItemWeapon_C|GetAccSightObj _weapon_3))
  (bind _sight (Variables|/Game/Blueprints/Items/Equipments/ItemWeapon.ItemWeapon_C|GetSight _weapon))
  (bind _accsightobj_2 (Variables|/Game/Blueprints/Items/Equipments/ItemWeapon.ItemWeapon_C|GetAccSightObj _weapon_2))
  (Utilities|FlowControl|Sequence
    (:then_0
      ;[1 1 1] Set The Camera Active States and model visibility
      (Rendering|SetVisibility (Variables|Default|GetFPSArm) IsFirst true)
      (Components|Activation|SetActive (Variables|Default|GetFPSCamera) IsFirst false)
      (Rendering|SetVisibility (Variables|Character|GetMesh) (not IsFirst) true)
      (Components|Activation|SetActive (Variables|Default|GetCamera) (not IsFirst) false))
    (:then_1
      ;[1 1 1] Weapons Are Attached To Character Models Or Arms
      (Transformation|SetActorTransform (Default|GetHoldGun (Variables|Default|GetMyPlayerStateRef)) (Math|Transform|SelectTransform (Transformation|GetSocketTransform (Variables|Default|GetFPSArm) "WeaponSocket" "RTS_World") (Transformation|GetSocketTransform (Variables|Character|GetMesh) (Default|CalculateHoldGunSocket (.AsMy%20Player%20Controller (Utilities|Casting|CastToMyPlayerController (Game|GetPlayerController 0)))) "RTS_World") IsFirst))
      (Transformation|AttachComponentToComponent (Default|GetHoldGun (Variables|Default|GetMyPlayerStateRef)) (select IsFirst (Variables|Default|GetFPSArm) (Variables|Character|GetMesh)) (select IsFirst "WeaponSocket" (Default|CalculateHoldGunSocket (.AsMy%20Player%20Controller (Utilities|Casting|CastToMyPlayerController (Game|GetPlayerController 0))))) "SnapToTarget" "KeepWorld" "KeepRelative" true)
      (Rendering|SetVisibility (Variables|/Game/Blueprints/Items/Equipments/ItemWeapon.ItemWeapon_C|GetSkeletalMesh (Default|GetHoldGun (Variables|Default|GetMyPlayerStateRef))) true true))
    (:then_2
      ;[1 1 1] If Equipped With 4x Scope, Set Sight model, Camera FOV  And Hide the Arm Model
      (Utilities|IsValid _accsightobj
        (:Is%20Valid
          (if (Utilities|Name|Equal(Name) (Variables|/Game/Blueprints/Items/ItemBase.ItemBase_C|GetID _accsightobj) "18")
            (if IsFirst
              (Transformation|SetRelativeScale3D _sight "0.100000,1.000000,1.000000")
              (Camera|SetFieldOfView _fpscamera 28.0)
              (Rendering|SetVisibility (Variables|Default|GetFPSArm) false false)
              (else
                (Transformation|SetRelativeScale3D _sight "1.000000,1.000000,1.000000")
                (Camera|SetFieldOfView _fpscamera 9e+01)))))))
    (:then_3
      ;[1 1 1] Set Arm Location
      (if IsFirst
        (Utilities|FlowControl|Sequence
          (:then_0
            (LocalVariables|SetWeaponID (Variables|/Game/Blueprints/Items/ItemBase.ItemBase_C|GetID (Default|GetHoldGun (Variables|Default|GetMyPlayerStateRef))))
            (Utilities|IsValid _accsightobj_2
              (:Is%20Valid
                (LocalVariables|SetSightID (Variables|/Game/Blueprints/Items/ItemBase.ItemBase_C|GetID _accsightobj_2)))
              (:Is%20Not%20Valid
                (LocalVariables|SetSightID "0"))))
          (:then_1
            (bind _returnvalue (Utilities|GetDataTableRow "/Game/Blueprints/Datas/DataTable/Aiming/DT_ArmsLocation.DT_ArmsLocation" (Utilities|String|StringToName (Utilities|String|Append (Utilities|String|ToString(Name) (LocalVariables|GetWeaponID)) "_" (Utilities|String|ToString(Name) (LocalVariables|GetSightID)))))
              (:then
                (Transformation|SetRelativeLocation (Variables|Default|GetFPSArm) (Utilities|Struct|BreakST_ArmsLocation _returnvalue) false false)))))))
    (:then_4
      ;[1 1 1] In The Third Person, the display of hair is hidden if a helmet is equipped
      (for _array_element (Default|GetEquipments (Variables|Default|GetMyPlayerStateRef))
        (if (and (Utilities|Enum|Equal(Enum) (Variables|/Game/Blueprints/Items/ItemBase.ItemBase_C|GetItemType _array_element) "NewEnumerator5") (not IsFirst))
          (Rendering|SetVisibility (Variables|Default|GetSKM_Hair) false true))))))

(fn SetIsSightAiming
  (params (IsSightAiming :type Boolean))
  (bind _myplayerstateref (Variables|Default|GetMyPlayerStateRef))
  (bind _weapon (Default|GetHoldGun _myplayerstateref))
  (bind _output_get (Variables|CharacterState|SetisSightAiming IsSightAiming))
  (if _output_get
    (Components|Timeline|SetPlayRate (Variables|Default|GetTL_HoldAiming) 2.0)
    (Variables|/Game/Blueprints/Items/Equipments/ItemWeapon.ItemWeapon_C|SetCanPlayFiringFlash _weapon false)
    (else
      (Variables|/Game/Blueprints/Items/Equipments/ItemWeapon.ItemWeapon_C|SetCanPlayFiringFlash _weapon true))))