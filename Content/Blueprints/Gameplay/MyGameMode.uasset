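; Game mode that scatters random pickup loot across the map at BeginPlay and passes the spawned items to the player controller.
; At each data-table location it spawns an ItemGroup, rolls unique item types and weighted IDs using percent-expanded arrays, then places pickups at unused group transforms.
; Weapons add matching ammo in place of a non-weapon item.
; RandomRoute, uncalled here, returns high-altitude endpoints on two different boundary lines from the game instance.
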(event EventBeginPlay
  (Utilities|FlowControl|Sequence ; testing sequence
    (:then_0
      (Variables|Default|SetMyGameInstanceRef (.AsMy%20Game%20Instance (Utilities|Casting|CastToMyGameInstance (Game|GetGameInstance))))
      (bind _items (GenerateItems|GenerateItems))
      (Default|SetPickupItems (.AsMy%20Player%20Controller (Utilities|Casting|CastToMyPlayerController (Game|GetPlayerController 0))) _items))))

(event EventTick
  (params (DeltaSeconds :type Float%20%28single-precision%29)))

(fn ConstructionScript)

(fn GenerateItems
  ;[1 1 1] get all item group locations.
  (bind _outrownames (DataTable|GetDataTableRowNames "/Game/Blueprints/Datas/DataTable/Items/DT_ItemGroupLocation.DT_ItemGroupLocation"))
  (for _array_element _outrownames
    (bind _returnvalue (Utilities|GetDataTableRow "/Game/Blueprints/Datas/DataTable/Items/DT_ItemGroupLocation.DT_ItemGroupLocation" _array_element)
      (:then
        ;[1 1 1] Spawn an item group actor
        (bind _returnvalue_2 (Game|SpawnActorfromClass "/Game/Blueprints/Items/ItemGroup.ItemGroup_C" (Math|Transform|MakeTransform (Utilities|Struct|BreakST_ItemGroupLocation _returnvalue)) "Undefined" 0 0))
        (LocalVariables|SetItemGroupRef _returnvalue_2)
        ;[1 1 1] Number of random items
        (bind _number (GenerateItems|RandomItemNumber))
        (for _index (range 1 _number)
          ;[1 1 1] Random Items type
          (bind _itemtype (GenerateItems|RandomItemType :!label _label))
          ;;[1 1 1] Type of item cannot repeat
          (if (== (Utilities|Array|FindItem (LocalVariables|GetItemsTypeArr) _itemtype) -1)
            (Utilities|Array|Add (LocalVariables|GetItemsTypeArr) _itemtype)
            (else
              (goto _label))))
        ;[1 1 1] Random Item ID
        (for _array_element_2 (LocalVariables|GetItemsTypeArr)
          (bind _item (GenerateItems|RandomItemID _array_element_2))
          (Utilities|Array|Add (LocalVariables|GetItemsIDArr) _item))
        (Utilities|Array|Clear (LocalVariables|GetItemsTypeArr))
        ;[1 1 1] Generating ammo for corresponding weapon type
        ;;[1 1 1] Find Weapon Item
        (for _array_element_3 (LocalVariables|GetItemsIDArr)
          (if (Utilities|Enum|Equal(Enum) (.Type (Utilities|Struct|BreakST_ItemTypeAndID _array_element_3)) "NewEnumerator0")
            ;;[1 1 1] Create Ammo
            (bind _returnvalue_3 (Utilities|GetDataTableRow "/Game/Blueprints/Datas/DataTable/Items/DT_Item_Weapon.DT_Item_Weapon" (.ID (Utilities|Struct|BreakST_ItemTypeAndID _array_element_3)))
              (:then
                (Utilities|Array|Add (LocalVariables|GetItemsIDArr) (Utilities|Struct|MakeST_ItemTypeAndID "NewEnumerator2" (Utilities|Struct|BreakST_Item_Weapon _returnvalue_3)))
                ;;[1 1 1] Remove an Item
                (bind (_array_element_4 _array_index) (Utilities|Array|ForEachLoopwithBreak (LocalVariables|GetItemsIDArr) :!label _label_2)
                  (:LoopBody
                    (if (Utilities|Enum|NotEqual(Enum) (.Type (Utilities|Struct|BreakST_ItemTypeAndID _array_element_4)) "NewEnumerator0")
                      (Utilities|Array|RemoveIndex (LocalVariables|GetItemsIDArr) _array_index)
                      (goto _label_2 Break))))))))
        ;[1 1 1] Loop all items ready to be generated
        (for _array_element_5 (LocalVariables|GetItemsIDArr)
          (LocalVariables|SetSpawnType (.Type (Utilities|Struct|BreakST_ItemTypeAndID _array_element_5)))
          (LocalVariables|SetSpawnID (.ID (Utilities|Struct|BreakST_ItemTypeAndID _array_element_5)))
          (Utilities|FlowControl|Sequence
            (:then_0
              ;[1 1 1] Randomize Location
              (bind _location (GenerateItems|RandomLocation (Default|GetAllTransform (LocalVariables|GetItemGroupRef)) :!label _label_3))
              (if (== (Utilities|Array|FindItem (LocalVariables|GetUsedLocations) _location) -1)
                (bind _output_get (LocalVariables|SetSpawnLocation _location))
                (Utilities|Array|Add (LocalVariables|GetUsedLocations) _output_get)
                (else
                  (goto _label_3))))
            (:then_1
              ;[1 1 1] Spawn Actor.
              (switch Utilities|FlowControl|Switch|SwitchonE_ItemType (LocalVariables|GetSpawnType)
                (:NewEnumerator0
                  (bind _returnvalue_4 (Game|SpawnActorfromClass "/Game/Blueprints/Items/Pickup/PickupWeapon.PickupWeapon_C" (LocalVariables|GetSpawnLocation) "Undefined" 0 0 (LocalVariables|GetSpawnID) (Default|GenerateSN (Variables|Default|GetMyGameInstanceRef)) 1 0))
                  (Utilities|Array|Add (LocalVariables|GetItemsObject) _returnvalue_4))
                (:NewEnumerator1
                  (bind _returnvalue_5 (Game|SpawnActorfromClass "/Game/Blueprints/Items/Pickup/PickupWeaponAcc.PickupWeaponAcc_C" (LocalVariables|GetSpawnLocation) "Undefined" 0 (LocalVariables|GetSpawnID) (Default|GenerateSN (Variables|Default|GetMyGameInstanceRef)) 1 0))
                  (Utilities|Array|Add (LocalVariables|GetItemsObject) _returnvalue_5))
                (:NewEnumerator2
                  (bind _returnvalue_6 (Game|SpawnActorfromClass "/Game/Blueprints/Items/Pickup/PickupAmmo.PickupAmmo_C" (LocalVariables|GetSpawnLocation) "Undefined" 0 (LocalVariables|GetSpawnID) (Default|GenerateSN (Variables|Default|GetMyGameInstanceRef)) 0 0))
                  (Utilities|Array|Add (LocalVariables|GetItemsObject) _returnvalue_6))
                (:NewEnumerator3
                  (bind _returnvalue_7 (Game|SpawnActorfromClass "/Game/Blueprints/Items/Pickup/PickupHealth.PickupHealth_C" (LocalVariables|GetSpawnLocation) "Undefined" 0 (LocalVariables|GetSpawnID) (Default|GenerateSN (Variables|Default|GetMyGameInstanceRef)) 1 0))
                  (Utilities|Array|Add (LocalVariables|GetItemsObject) _returnvalue_7))
                (:NewEnumerator4
                  (bind _returnvalue_8 (Game|SpawnActorfromClass "/Game/Blueprints/Items/Pickup/PickupBoost.PickupBoost_C" (LocalVariables|GetSpawnLocation) "Undefined" 0 (LocalVariables|GetSpawnID) (Default|GenerateSN (Variables|Default|GetMyGameInstanceRef)) 1 0))
                  (Utilities|Array|Add (LocalVariables|GetItemsObject) _returnvalue_8))
                (:NewEnumerator5
                  (bind _returnvalue_9 (Game|SpawnActorfromClass "/Game/Blueprints/Items/Pickup/PickupEquipment.PickupEquipment_C" (LocalVariables|GetSpawnLocation) "Undefined" 0 (LocalVariables|GetSpawnID) (Default|GenerateSN (Variables|Default|GetMyGameInstanceRef)) 1 0 :!label _label_4))
                  (Utilities|Array|Add (LocalVariables|GetItemsObject) _returnvalue_9))
                (:NewEnumerator6
                  (goto _label_4))
                (:NewEnumerator7
                  (goto _label_4))
                (:NewEnumerator8
                  (bind _returnvalue_10 (Game|SpawnActorfromClass "/Game/Blueprints/Items/Pickup/pICKUPfASHION.PickupFashion_C" (LocalVariables|GetSpawnLocation) "Undefined" 0 (LocalVariables|GetSpawnID) (Default|GenerateSN (Variables|Default|GetMyGameInstanceRef)) 0 0))
                  (Utilities|Array|Add (LocalVariables|GetItemsObject) _returnvalue_10))))))
        (Utilities|Array|Clear (LocalVariables|GetItemsIDArr)))))
  (return (LocalVariables|GetItemsObject)))

(fn RandomItemNumber
  (bind _arr (LocalVariables|GetArr))
  (bind _outrownames (DataTable|GetDataTableRowNames "/Game/Blueprints/Datas/DataTable/ItemGeneration/DT_NumberProbability.DT_NumberProbability"))
  (for _array_element _outrownames
    (bind _returnvalue (Utilities|GetDataTableRow "/Game/Blueprints/Datas/DataTable/ItemGeneration/DT_NumberProbability.DT_NumberProbability" _array_element)
      (:then
        (for _index (range 1 (.Percent (Utilities|Struct|BreakST_NumberProbability _returnvalue)))
          (Utilities|Array|Add (LocalVariables|GetArr) (.Number (Utilities|Struct|BreakST_NumberProbability _returnvalue)))))))
  (Utilities|Array|Shuffle _arr)
  (return (Utilities|Array|Get(acopy) _arr (Math|Random|RandomIntegerinRange 0 99))))

(fn RandomItemType
  (bind _arr (LocalVariables|GetArr))
  (bind _outrownames (DataTable|GetDataTableRowNames "/Game/Blueprints/Datas/DataTable/ItemGeneration/DT_ItemTypeProbability.DT_ItemTypeProbability"))
  (for _array_element _outrownames
    (bind _returnvalue (Utilities|GetDataTableRow "/Game/Blueprints/Datas/DataTable/ItemGeneration/DT_ItemTypeProbability.DT_ItemTypeProbability" _array_element)
      (:then
        (for _index (range 1 (.Percent (Utilities|Struct|BreakST_ItemTypeProbability _returnvalue)))
          (Utilities|Array|Add (LocalVariables|GetArr) (.Type (Utilities|Struct|BreakST_ItemTypeProbability _returnvalue)))))))
  (Utilities|Array|Shuffle _arr)
  (return (Utilities|Array|Get(acopy) _arr (Math|Random|RandomIntegerinRange 0 99))))

(fn RandomItemID
  (params (ItemType :type E_ItemType%20Enum :default "NewEnumerator0"))
  (bind _arr (LocalVariables|GetArr))
  (Utilities|FlowControl|Sequence
    (:then_0
      (switch Utilities|FlowControl|Switch|SwitchonE_ItemType ItemType
        (:NewEnumerator0
          (bind _outrownames (DataTable|GetDataTableRowNames "/Game/Blueprints/Datas/DataTable/Items/DT_Item_Weapon.DT_Item_Weapon"))
          (for _array_element _outrownames
            (bind _returnvalue (Utilities|GetDataTableRow "/Game/Blueprints/Datas/DataTable/Items/DT_Item_Weapon.DT_Item_Weapon" _array_element)
              (:then
                (for _index (range 1 (Utilities|Struct|BreakST_Item_Weapon _returnvalue))
                  (Utilities|Array|Add (LocalVariables|GetArr) (Utilities|Struct|MakeST_ItemTypeAndID "NewEnumerator0" _array_element)))))))
        (:NewEnumerator1
          (bind _outrownames_2 (DataTable|GetDataTableRowNames "/Game/Blueprints/Datas/DataTable/Items/DT_Item_WeaponAcc.DT_Item_WeaponAcc"))
          (for _array_element_2 _outrownames_2
            (Utilities|Array|Add (LocalVariables|GetArr) (Utilities|Struct|MakeST_ItemTypeAndID "NewEnumerator1" _array_element_2))))
        (:NewEnumerator2
          (bind _outrownames_3 (DataTable|GetDataTableRowNames "/Game/Blueprints/Datas/DataTable/Items/DT_Item_Ammo.DT_Item_Ammo"))
          (for _array_element_3 _outrownames_3
            (bind _returnvalue_2 (Utilities|GetDataTableRow "/Game/Blueprints/Datas/DataTable/Items/DT_Item_Ammo.DT_Item_Ammo" _array_element_3)
              (:then
                (for _index_2 (range 1 (Utilities|Struct|BreakST_ItemAmmo _returnvalue_2))
                  (Utilities|Array|Add (LocalVariables|GetArr) (Utilities|Struct|MakeST_ItemTypeAndID "NewEnumerator2" _array_element_3)))))))
        (:NewEnumerator3
          (bind _outrownames_4 (DataTable|GetDataTableRowNames "/Game/Blueprints/Datas/DataTable/Items/DT_Item_Health.DT_Item_Health"))
          (for _array_element_4 _outrownames_4
            (bind _returnvalue_3 (Utilities|GetDataTableRow "/Game/Blueprints/Datas/DataTable/Items/DT_Item_Health.DT_Item_Health" _array_element_4)
              (:then
                (for _index_3 (range 1 (Utilities|Struct|BreakST_Item_Health _returnvalue_3))
                  (Utilities|Array|Add (LocalVariables|GetArr) (Utilities|Struct|MakeST_ItemTypeAndID "NewEnumerator3" _array_element_4)))))))
        (:NewEnumerator4
          (bind _outrownames_5 (DataTable|GetDataTableRowNames "/Game/Blueprints/Datas/DataTable/Items/DT_Item_Boost.DT_Item_Boost"))
          (for _array_element_5 _outrownames_5
            (bind _returnvalue_4 (Utilities|GetDataTableRow "/Game/Blueprints/Datas/DataTable/Items/DT_Item_Boost.DT_Item_Boost" _array_element_5)
              (:then
                (for _index_4 (range 1 (.ProbabilityPercent (Utilities|Struct|BreakST_Item_Boost _returnvalue_4)))
                  (Utilities|Array|Add (LocalVariables|GetArr) (Utilities|Struct|MakeST_ItemTypeAndID "NewEnumerator4" _array_element_5)))))))
        (:NewEnumerator5
          (bind _outrownames_6 (DataTable|GetDataTableRowNames "/Game/Blueprints/Datas/DataTable/Items/DT_Item_Equipment.DT_Item_Equipment"))
          (for _array_element_6 _outrownames_6
            (bind _returnvalue_5 (Utilities|GetDataTableRow "/Game/Blueprints/Datas/DataTable/Items/DT_Item_Equipment.DT_Item_Equipment" _array_element_6)
              (:then
                (if (Utilities|Enum|Equal(Enum) (.Type (Utilities|Struct|BreakST_Item_Equipment _returnvalue_5)) "NewEnumerator5")
                  (for _index_5 (range 1 (.ProbabilityPercent (Utilities|Struct|BreakST_Item_Equipment _returnvalue_5)))
                    (Utilities|Array|Add (LocalVariables|GetArr) (Utilities|Struct|MakeST_ItemTypeAndID "NewEnumerator5" _array_element_6))))))))
        (:NewEnumerator6
          (bind _outrownames_7 (DataTable|GetDataTableRowNames "/Game/Blueprints/Datas/DataTable/Items/DT_Item_Equipment.DT_Item_Equipment"))
          (for _array_element_7 _outrownames_7
            (bind _returnvalue_6 (Utilities|GetDataTableRow "/Game/Blueprints/Datas/DataTable/Items/DT_Item_Equipment.DT_Item_Equipment" _array_element_7)
              (:then
                (if (Utilities|Enum|Equal(Enum) (.Type (Utilities|Struct|BreakST_Item_Equipment _returnvalue_6)) "NewEnumerator6")
                  (for _index_6 (range 1 (.ProbabilityPercent (Utilities|Struct|BreakST_Item_Equipment _returnvalue_6)))
                    (Utilities|Array|Add (LocalVariables|GetArr) (Utilities|Struct|MakeST_ItemTypeAndID "NewEnumerator6" _array_element_7))))))))
        (:NewEnumerator7
          (bind _outrownames_8 (DataTable|GetDataTableRowNames "/Game/Blueprints/Datas/DataTable/Items/DT_Item_Equipment.DT_Item_Equipment"))
          (for _array_element_8 _outrownames_8
            (bind _returnvalue_7 (Utilities|GetDataTableRow "/Game/Blueprints/Datas/DataTable/Items/DT_Item_Equipment.DT_Item_Equipment" _array_element_8)
              (:then
                (if (Utilities|Enum|Equal(Enum) (.Type (Utilities|Struct|BreakST_Item_Equipment _returnvalue_7)) "NewEnumerator7")
                  (for _index_7 (range 1 (.ProbabilityPercent (Utilities|Struct|BreakST_Item_Equipment _returnvalue_7)))
                    (Utilities|Array|Add (LocalVariables|GetArr) (Utilities|Struct|MakeST_ItemTypeAndID "NewEnumerator7" _array_element_8))))))))
        (:NewEnumerator8
          (bind _outrownames_9 (DataTable|GetDataTableRowNames "/Game/Blueprints/Datas/DataTable/Items/DT_Item_Fashion.DT_Item_Fashion"))
          (for _array_element_9 _outrownames_9
            (if (and (Utilities|Name|NotEqual(Name) _array_element_9 "1") (Utilities|Name|NotEqual(Name) _array_element_9 "4"))
              (Utilities|Array|Add (LocalVariables|GetArr) (Utilities|Struct|MakeST_ItemTypeAndID "NewEnumerator8" _array_element_9)))))))
    (:then_1
      (Utilities|Array|Shuffle _arr)
      (return (Utilities|Array|Get(acopy) _arr (Math|Random|RandomIntegerinRange 0 (- (Utilities|Array|Length (LocalVariables|GetArr)) 1)))))))

(fn RandomLocation
  (params (Available :type Array%20of%20Transforms))
  (return (Utilities|Array|Get(acopy) Available (Math|Random|RandomIntegerinRange 0 (- (Utilities|Array|Length Available) 1)))))

(fn RandomRoute
  (bind _mygameinstanceref (Variables|Default|GetMyGameInstanceRef))
  (bind _mygameinstanceref_2 (Variables|Default|GetMyGameInstanceRef))
  (bind _mygameinstanceref_3 (Variables|Default|GetMyGameInstanceRef))
  (bind _mygameinstanceref_4 (Variables|Default|GetMyGameInstanceRef))
  (bind _mygameinstanceref_5 (Variables|Default|GetMyGameInstanceRef))
  (bind _mygameinstanceref_6 (Variables|Default|GetMyGameInstanceRef))
  (bind _mygameinstanceref_7 (Variables|Default|GetMyGameInstanceRef))
  (bind _mygameinstanceref_8 (Variables|Default|GetMyGameInstanceRef))
  (Utilities|FlowControl|Sequence
    (:then_0
      ;[1 1 1] Random Start Pos
      (Utilities|FlowControl|Sequence
        (:then_0
          (LocalVariables|SetStartIndex (Math|Random|RandomIntegerinRange 1 4))
          (if (== (LocalVariables|GetStartIndex) 1)
            (LocalVariables|SetLineMin (Variables|/Game/Blueprints/Gameplay/MyGameInstance.MyGameInstance_C|GetLine1Min _mygameinstanceref_4))
            (LocalVariables|SetLineMax (Variables|/Game/Blueprints/Gameplay/MyGameInstance.MyGameInstance_C|GetLine1Max _mygameinstanceref_4))
            (elif (== (LocalVariables|GetStartIndex) 2)
              (LocalVariables|SetLineMin (Variables|/Game/Blueprints/Gameplay/MyGameInstance.MyGameInstance_C|GetLine2Min _mygameinstanceref_5))
              (LocalVariables|SetLineMax (Variables|/Game/Blueprints/Gameplay/MyGameInstance.MyGameInstance_C|GetLine2Max _mygameinstanceref_5))
              (elif (== (LocalVariables|GetStartIndex) 3)
                (LocalVariables|SetLineMin (Variables|/Game/Blueprints/Gameplay/MyGameInstance.MyGameInstance_C|GetLine3Min _mygameinstanceref_6))
                (LocalVariables|SetLineMax (Variables|/Game/Blueprints/Gameplay/MyGameInstance.MyGameInstance_C|GetLine3Max _mygameinstanceref_6))
                (elif (== (LocalVariables|GetStartIndex) 4)
                  (LocalVariables|SetLineMin (Variables|/Game/Blueprints/Gameplay/MyGameInstance.MyGameInstance_C|GetLine4Min _mygameinstanceref_7))
                  (LocalVariables|SetLineMax (Variables|/Game/Blueprints/Gameplay/MyGameInstance.MyGameInstance_C|GetLine4Max _mygameinstanceref_7)))))))
        (:then_1
          (LocalVariables|SetStartVector (Math|Vector|MakeVector (Math|Random|RandomFloatinRange (.X (Math|Vector2D|BreakVector2D (LocalVariables|GetLineMin))) (.X (Math|Vector2D|BreakVector2D (LocalVariables|GetLineMax)))) (Math|Random|RandomFloatinRange (.Y (Math|Vector2D|BreakVector2D (LocalVariables|GetLineMin))) (.Y (Math|Vector2D|BreakVector2D (LocalVariables|GetLineMax)))) 1.5e+05)))))
    (:then_1
      ;[1 1 1] Random end pos
      (Utilities|FlowControl|Sequence
        (:then_0
          ;;[1 1 1] Start Index and End index can't be on the same line
          (bind _output_get (LocalVariables|SetEndIndex (Math|Random|RandomIntegerinRange 1 4) :!label _label))
          (if (== _output_get (LocalVariables|GetStartIndex))
            (goto _label)
            (elif (== (LocalVariables|GetEndIndex) 1)
              (LocalVariables|SetLineMin (Variables|/Game/Blueprints/Gameplay/MyGameInstance.MyGameInstance_C|GetLine1Min _mygameinstanceref_8))
              (LocalVariables|SetLineMax (Variables|/Game/Blueprints/Gameplay/MyGameInstance.MyGameInstance_C|GetLine1Max _mygameinstanceref_8))
              (elif (== (LocalVariables|GetEndIndex) 2)
                (LocalVariables|SetLineMin (Variables|/Game/Blueprints/Gameplay/MyGameInstance.MyGameInstance_C|GetLine2Min _mygameinstanceref_3))
                (LocalVariables|SetLineMax (Variables|/Game/Blueprints/Gameplay/MyGameInstance.MyGameInstance_C|GetLine2Max _mygameinstanceref_3))
                (elif (== (LocalVariables|GetEndIndex) 3)
                  (LocalVariables|SetLineMin (Variables|/Game/Blueprints/Gameplay/MyGameInstance.MyGameInstance_C|GetLine3Min _mygameinstanceref_2))
                  (LocalVariables|SetLineMax (Variables|/Game/Blueprints/Gameplay/MyGameInstance.MyGameInstance_C|GetLine3Max _mygameinstanceref_2))
                  (elif (== (LocalVariables|GetEndIndex) 4)
                    (LocalVariables|SetLineMin (Variables|/Game/Blueprints/Gameplay/MyGameInstance.MyGameInstance_C|GetLine4Min _mygameinstanceref))
                    (LocalVariables|SetLineMax (Variables|/Game/Blueprints/Gameplay/MyGameInstance.MyGameInstance_C|GetLine4Max _mygameinstanceref))))))))
        (:then_1
          (LocalVariables|SetEndVector (Math|Vector|MakeVector (Math|Random|RandomFloatinRange (.X (Math|Vector2D|BreakVector2D (LocalVariables|GetLineMin))) (.X (Math|Vector2D|BreakVector2D (LocalVariables|GetLineMax)))) (Math|Random|RandomFloatinRange (.Y (Math|Vector2D|BreakVector2D (LocalVariables|GetLineMin))) (.Y (Math|Vector2D|BreakVector2D (LocalVariables|GetLineMax)))) 1.5e+05)))))
    (:then_2
      (return (LocalVariables|GetStartVector) (LocalVariables|GetEndVector)))))